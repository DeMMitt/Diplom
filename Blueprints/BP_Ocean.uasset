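; BP_Ocean is the sea actor, telling fish when they are in water and triggering the fishing rod's splash sound.
; On BeginPlay it flags the physics volume returned by its WaterVolume component as water.
; That component's overlap events switch each BP_FishBase in or out of its water state.
; An entering BP_FishingRod plays its plop cue unless its Caught flag is set.
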(event `self.ReceiveBeginPlay`
  (set `PhysicsVolume.bWaterVolume` true (`SceneComponent.GetPhysicsVolume` (`self.WaterVolume`))))

(event `self.WaterVolume.OnComponentBeginOverlap`
  (params (OverlappedComponent :type "PrimitiveComponent Object Reference") (OtherActor :type "Actor Object Reference") (OtherComp :type "PrimitiveComponent Object Reference") (OtherBodyIndex :type Integer) (bFromSweep :type Boolean) (SweepResult :type "HitResult Structure (by ref)"))
  (bind _asbp_fish_base (cast `/Game/AdvancedFishingTemplate/Blueprints/BP_FishBase` OtherActor)
    (:`then`
      (`/Game/AdvancedFishingTemplate/Blueprints/BP_FishBase.SetInWater` _asbp_fish_base true))
    (:`CastFailed`
      (bind _asbp_fishing_rod (cast `/Game/AdvancedFishingTemplate/Blueprints/BP_FishingRod` OtherActor))
      (if (not (`/Game/AdvancedFishingTemplate/Blueprints/BP_FishingRod.Caught` _asbp_fishing_rod))
        (`AudioComponent.Play` (`/Game/AdvancedFishingTemplate/Blueprints/BP_FishingRod.Plop_Cue` _asbp_fishing_rod) 0.0)))))

(event `self.WaterVolume.OnComponentEndOverlap`
  (params (OverlappedComponent :type "PrimitiveComponent Object Reference") (OtherActor :type "Actor Object Reference") (OtherComp :type "PrimitiveComponent Object Reference") (OtherBodyIndex :type Integer))
  (bind _asbp_fish_base (cast `/Game/AdvancedFishingTemplate/Blueprints/BP_FishBase` OtherActor))
  (`/Game/AdvancedFishingTemplate/Blueprints/BP_FishBase.SetInWater` _asbp_fish_base false))

(fn `UserConstructionScript`)