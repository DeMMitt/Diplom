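; Player controller for the fishing game that creates the HUD and bucket widgets and handles fishing input.
; Mouse buttons drive reel up/down on the character's child-actor fishing rod, Shift+click casts near the end of a montage, and holding Tab shows the bucket.
; Tick polls the rod's current fish to toggle the caught-fish widget and input mode, and slows the character's play rate for heavier fish.
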(event `self.ReceiveBeginPlay`
  ;[0 0 1] Getting Character Reference
  (bind _asbp_fishing_player_character (cast `/Game/AdvancedFishingTemplate/Blueprints/BP_FishingPlayerCharacter` (`GameplayStatics.GetPlayerCharacter` 0)))
  (set `self.CharacterRef` _asbp_fishing_player_character)
  ;[0 0 1] Adding HUD
  (bind _returnvalue (`|CreateWidget` "/Game/AdvancedFishingTemplate/Blueprints/Widgets/HUD.HUD_C"))
  (bind _output_get (set `self.W_HUD` _returnvalue))
  (`UserWidget.AddToViewport` _output_get 0)
  ;[0 0 1] Adding Bucket Widget
  (bind _returnvalue_2 (`|CreateWidget` "/Game/AdvancedFishingTemplate/Blueprints/Widgets/Bucket.Bucket_C"))
  (bind _output_get_2 (set `self.W_Bucket` _returnvalue_2))
  (`UserWidget.AddToViewport` _output_get_2 0)
  ;[0 0 1] Bucket Slot Reference
  (bind _returnvalue_3 (`|CreateWidget` "/Game/AdvancedFishingTemplate/Blueprints/Widgets/BucketSlot.BucketSlot_C"))
  (set `self.W_BucketSlot` _returnvalue_3))

(event `Key|RightMouseButton`
  (params (Key :type "Key Structure"))
  (bind _characterref (`self.CharacterRef`))
  (bind _childactor (`ChildActorComponent.ChildActor` (`/Game/AdvancedFishingTemplate/Blueprints/BP_FishingPlayerCharacter.FishingRod` _characterref)))
  ;[1 0 0] Reel Down
  (:`Pressed`
    (set `/Game/AdvancedFishingTemplate/Blueprints/BP_FishingPlayerCharacter.ReelDown` true _characterref)
    (bind _asbp_fishing_rod (cast `/Game/AdvancedFishingTemplate/Blueprints/BP_FishingRod` _childactor))
    (`/Game/AdvancedFishingTemplate/Blueprints/BP_FishingRod.ReelDown` _asbp_fishing_rod))
  (:`Released`
    (set `/Game/AdvancedFishingTemplate/Blueprints/BP_FishingPlayerCharacter.ReelDown` false _characterref)
    (bind _asbp_fishing_rod_2 (cast `/Game/AdvancedFishingTemplate/Blueprints/BP_FishingRod` _childactor))
    (`/Game/AdvancedFishingTemplate/Blueprints/BP_FishingRod.ReelDownStop` _asbp_fishing_rod_2)))

(event `Key|Tab`
  (params (Key :type "Key Structure"))
  (bind _returnvalue (`GameplayStatics.GetPlayerController` 0))
  (bind _w_bucket (`self.W_Bucket`))
  ;[1 0 0] Show Bucket
  (:`Pressed`
    (`Widget.SetVisibility` _w_bucket "Visible")
    (set `self.bShowMouseCursor` true)
    (`WidgetBlueprintLibrary.SetInputMode_GameAndUIEx` _returnvalue _w_bucket))
  (:`Released`
    (`Widget.SetVisibility` _w_bucket "Hidden")
    (set `self.bShowMouseCursor` false)
    (`WidgetBlueprintLibrary.SetInputMode_GameOnly` _returnvalue)))

(event `Key|LeftMouseButton`
  (params (Key :type "Key Structure"))
  (bind _characterref (`self.CharacterRef`))
  (bind _childactor (`ChildActorComponent.ChildActor` (`/Game/AdvancedFishingTemplate/Blueprints/BP_FishingPlayerCharacter.FishingRod` _characterref)))
  ;[1 0 0] Reel Up
  (:`Pressed`
    (set `/Game/AdvancedFishingTemplate/Blueprints/BP_FishingPlayerCharacter.ReelUp` true _characterref)
    (bind _asbp_fishing_rod (cast `/Game/AdvancedFishingTemplate/Blueprints/BP_FishingRod` _childactor))
    (`/Game/AdvancedFishingTemplate/Blueprints/BP_FishingRod.ReelUp` _asbp_fishing_rod))
  (:`Released`
    (set `/Game/AdvancedFishingTemplate/Blueprints/BP_FishingPlayerCharacter.ReelUp` false _characterref)
    (bind _asbp_fishing_rod_2 (cast `/Game/AdvancedFishingTemplate/Blueprints/BP_FishingRod` _childactor))
    (`/Game/AdvancedFishingTemplate/Blueprints/BP_FishingRod.ReelUpStop` _asbp_fishing_rod_2)))

(event `Key|Shift+LeftMouseButton`
  (params (Key :type "Key Structure"))
  ;[1 0 0] Cast
  (:`Pressed`
    (bind _returnvalue (`AnimInstance.Montage_Play` (`SkeletalMeshComponent.GetAnimInstance` (`Character.Mesh` (`self.CharacterRef`))) "/Game/AdvancedFishingTemplate/Animations/CastAnim_Montage.CastAnim_Montage" 2.0 "Duration" 0.0 true))
    (`KismetSystemLibrary.Delay` (- _returnvalue 0.5))
    (bind _asbp_fishing_rod (cast `/Game/AdvancedFishingTemplate/Blueprints/BP_FishingRod` (`ChildActorComponent.ChildActor` (`/Game/AdvancedFishingTemplate/Blueprints/BP_FishingPlayerCharacter.FishingRod` (`self.CharacterRef`)))))
    (`/Game/AdvancedFishingTemplate/Blueprints/BP_FishingRod.Cast` _asbp_fishing_rod)))

(event `self.ReceiveTick`
  (params (DeltaSeconds :type "Float (single-precision)"))
  (bind _returnvalue (`GameplayStatics.GetPlayerController` 0))
  (bind _characterref (`self.CharacterRef`))
  (bind _characterref_2 (`self.CharacterRef`))
  (bind _w_fishcaught (`self.W_FishCaught`))
  ;[0 1 0] If fish caught show fish Caught widget
  (bind _asbp_fishing_rod (cast `/Game/AdvancedFishingTemplate/Blueprints/BP_FishingRod` (`ChildActorComponent.ChildActor` (`/Game/AdvancedFishingTemplate/Blueprints/BP_FishingPlayerCharacter.FishingRod` (`self.CharacterRef`)))))
  (bind _currentfishref (`/Game/AdvancedFishingTemplate/Blueprints/BP_FishingRod.CurrentFishRef` _asbp_fishing_rod))
  (`/Engine/EditorBlueprintResources/StandardMacros.IsValid` _currentfishref
    (:`Is Valid`
      (`|ExecutionSequence`
        (:`then_0`
          (if (`/Game/AdvancedFishingTemplate/Blueprints/BP_FishBase.FishCaught` _currentfishref)
            (if (not (`/Game/AdvancedFishingTemplate/Blueprints/BP_FishingPlayerCharacter.CaughtWidgetOnScreen` (`self.CharacterRef`)))
              (bind _returnvalue_2 (`|CreateWidget` "/Game/AdvancedFishingTemplate/Blueprints/Widgets/FishCaught.FishCaught_C"))
              (set `self.W_FishCaught` _returnvalue_2)
              (`UserWidget.AddToViewport` (`self.W_FishCaught`) 1)
              (`WidgetBlueprintLibrary.SetInputMode_GameAndUIEx` _returnvalue (`self.W_FishCaught`))
              (set `PlayerController.bShowMouseCursor` true _returnvalue)
              (set `/Game/AdvancedFishingTemplate/Blueprints/BP_FishingPlayerCharacter.CaughtWidgetOnScreen` true _characterref))
            (else
              (`/Engine/EditorBlueprintResources/StandardMacros.IsValid` _w_fishcaught
                (:`Is Valid`
                  (`Widget.RemoveFromParent` _w_fishcaught)
                  (`WidgetBlueprintLibrary.SetInputMode_GameOnly` _returnvalue)
                  (set `PlayerController.bShowMouseCursor` false _returnvalue)
                  (set `/Game/AdvancedFishingTemplate/Blueprints/BP_FishingPlayerCharacter.CaughtWidgetOnScreen` false _characterref))))))
        (:`then_1`
          (bind ((`FishImage_21_99759A6D411D67324B6A8BA642D4596D` _fishimage) (`Weight_7_526CA6DA4A111688D6D74FA8AA5B035E` _weight)) (break `/Game/AdvancedFishingTemplate/Blueprints/FishDetails` (`/Game/AdvancedFishingTemplate/Blueprints/BP_FishBase.FishProperties` _currentfishref)))
          (if (> _weight 1.0)
            (bind _returnvalue_3 (/ _weight 10.0))
            (if (>= _returnvalue_3 1.0)
              (set `/Game/AdvancedFishingTemplate/Blueprints/BP_FishingPlayerCharacter.Playrate` 0.3 _characterref_2)
              (else
                (set `/Game/AdvancedFishingTemplate/Blueprints/BP_FishingPlayerCharacter.Playrate` (- 1.0 _returnvalue_3) _characterref_2)))
            (else
              (set `/Game/AdvancedFishingTemplate/Blueprints/BP_FishingPlayerCharacter.Playrate` 1.0 (`self.CharacterRef`) :!label _label))))))
    (:`Is Not Valid`
      (goto _label))))

(fn `UserConstructionScript`)